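; Zombie-mode player character that receives a Glock loadout on possession and adds health regen, bleed-out and teammate revives.
; The use button inside a revive trigger calls server events that restore the downed player's health, movement and HUD.
; A bleed-out timer function counts down a RepNotify counter shown on the overhead name widget.
; The downing logic that starts that timer is disconnected; OnDeath just marks death and asks the GameMode to check game over.
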(event Custom|ReviveButtonDown
  (bind _returnvalue (Pawn|GetController))
  ;[0 1 0] Revive and Interaction System
  (Variables|Interaction/Revive|SetUseButtonPressed? true)
  (if (Variables|PlayerVariables|GetShowHintstrings?)
    (Utilities|IsValid _returnvalue
      (:Is%20Valid
        (bind _asbp_zmplayer_controller (Utilities|Casting|CastToBP_ZMPlayerController _returnvalue))
        (Variables|PlayerVariables|SetMyPlayerController _asbp_zmplayer_controller)
        (if (not (Variables|Interaction/Revive|GetIsDowned?)) ; If your not downed then you revive others
          (if (Variables|Interaction/Revive|GetTouchingReviveTrigger?) ; Are You Reviving Or Interacting?
            (CallFunction|RevivingPlayer)))))))

(event Custom|ClientHideWeapon
  (Rendering|SetVisibility (Variables|Default|GetFreeAimSpringArm) false true)
  (Default|HideHUD (CallFunction|GetHDPlayerControllerBP))
  (bind _asbp_zmplayer_controller (Utilities|Casting|CastToBP_ZMPlayerController (Pawn|GetController)))
  (Default|PlayerDowned (Variables|/ZombieSurvival/Core/BP_ZMPlayerController.BP_ZMPlayerController_C|GetHUDWidgetReference _asbp_zmplayer_controller) true))

(event Custom|PlayerHasDied
  (bind _revivetrigger (Variables|Interaction/Revive|GetReviveTrigger))
  ;[0 1 0] Player Has Died. This will tell the Gamemode that you died and then either respawn, game over, or spectate.
  (Utilities|Time|ClearTimerbyFunctionName 0 "BleedOutTimer")
  (Utilities|IsValid _revivetrigger
    (:Is%20Valid
      (Actor|DestroyActor _revivetrigger))
    (:Is%20Not%20Valid
      _))
  (bind _asbp_zmplayer_controller (Utilities|Casting|CastToBP_ZMPlayerController (Pawn|GetController)))
  (Default|PassCharacterInfotoServer _asbp_zmplayer_controller))

(event Custom|ClientResetHealth
  (CallFunction|EventResetHealthEffect)
  (Rendering|SetVisibility (Variables|Default|GetFreeAimSpringArm) true true)
  (Default|ShowHUD (CallFunction|GetHDPlayerControllerBP))
  (bind _asbp_zmplayer_controller (Utilities|Casting|CastToBP_ZMPlayerController (Pawn|GetController)))
  (Default|PlayerDowned (Variables|/ZombieSurvival/Core/BP_ZMPlayerController.BP_ZMPlayerController_C|GetHUDWidgetReference _asbp_zmplayer_controller) false))

(event Custom|ShowReviveImage
  ;[0 1 0] Shows the Revive Image above your head for others to see that your downed.
  (bind _aswbp_player_name_above_widget (Utilities|Casting|CastToWBP_PlayerNameAboveWidget (UserInterface|GetUserWidgetObject (Variables|Default|GetPlayerNameWidget))))
  (Widget|SetVisibility (Variables|/ZombieSurvival/Blueprints/Widgets/WBP_PlayerNameAboveWidget.WBP_PlayerNameAboveWidget_C|GetReviveImage _aswbp_player_name_above_widget) "Visible"))

(event Custom|PlaySoundOnPlayer
  (params (SoundWave :type Sound%20Cue%20Object%20Reference))
  ;[1 1 0] Plays sound on player
  (Audio|PlaySoundatLocation SoundWave (Transformation|GetActorLocation) "0, 0, 0" 1.0 1.0 0.0 0 0 0))

(event Custom|HideReviveImage
  ;[0 1 0] Hides The Revive Image When Not Downed
  (bind _aswbp_player_name_above_widget (Utilities|Casting|CastToWBP_PlayerNameAboveWidget (UserInterface|GetUserWidgetObject (Variables|Default|GetPlayerNameWidget))))
  (Widget|SetVisibility (Variables|/ZombieSurvival/Blueprints/Widgets/WBP_PlayerNameAboveWidget.WBP_PlayerNameAboveWidget_C|GetReviveImage _aswbp_player_name_above_widget) "Hidden")
  (Appearance|SetColorandOpacity (Variables|/ZombieSurvival/Blueprints/Widgets/WBP_PlayerNameAboveWidget.WBP_PlayerNameAboveWidget_C|GetReviveText _aswbp_player_name_above_widget) (Utilities|Struct|MakeSlateColor (Variables|/ZombieSurvival/Blueprints/Widgets/WBP_PlayerNameAboveWidget.WBP_PlayerNameAboveWidget_C|GetGreen _aswbp_player_name_above_widget) "UseColor_Specified") :!class /Script/UMG.TextBlock))

(event Custom|ServerPauseBleedOutTime
  ;[0 1 0] Server Pause BleedOut Timer for Person Your Reviving
  (Class|KismetSystemLibrary|PauseTimer (Variables|Interaction/Revive|GetPlayerYourReviving) "BleedOutTimer")
  (Variables|Default|SetisBeingRevived? true))

(event Custom|HealthRegen
  ;[0 1 0] Health Regeration
  (Timeline|HealthRegenTimeline Play
    (:Update
      (if (Variables|PlayerVariables|GetHealthRegen?)
        (if (< (Variables|Default|GetHealth) (Variables|Default|GetMaxHealth))
          (bind _output_get (Variables|Default|SetHealth (Math|Float|Min(Float) (+ (Variables|Default|GetHealth) (Variables|PlayerVariables|GetHealthRegenRate)) (Variables|Default|GetMaxHealth))))
          (if (== _output_get (Variables|Default|GetMaxHealth))
            (Audio|Components|Audio|Stop (Variables|Default|GetHealthRegenTimeline))))))))

(event Custom|ServerRevivePlayer
  (bind _revivetrigger (Variables|Interaction/Revive|GetReviveTrigger))
  ;[0 1 0] Server Revive Player and Destroys the Revive Trigger
  (Variables|Default|SetHealth (Variables|Default|GetMaxHealth))
  (Variables|Interaction/Revive|SetBleedOutCounter (Variables|Interaction/Revive|GetBleedOutTime))
  (Variables|Interaction/Revive|SetIsDowned? false)
  (Variables|PlayerVariables|SetHealthRegen? true)
  (Utilities|Time|ClearandInvalidateTimerbyHandle (Variables|Interaction/Revive|GetBleedoutTimerHandle))
  (CallFunction|ClientResetHealth)
  (Pawn|Components|CharacterMovement|SetMovementMode (Variables|Character|GetCharacterMovement) "MOVE_Walking" 0)
  (CallFunction|HideReviveImage)
  (Utilities|IsValid _revivetrigger
    (:Is%20Valid
      (Actor|DestroyActor _revivetrigger))
    (:Is%20Not%20Valid
      _))
  (Utilities|FlowControl|Delay 2.0) ; Small delay Before allowing Damage Again
  (Variables|Default|SetbCanBeDamaged true))

(event Custom|PlaySoundCueOnPlayer
  (params (SoundWave :type Sound%20Cue%20Object%20Reference))
  ;[1 1 0] Plays sound on player
  (Audio|PlaySoundatLocation SoundWave (Transformation|GetActorLocation) "0, 0, 0" 1.0 1.0 0.0 0 0 0))

(event Custom|ServerUnPauseBleedOutTimer
  (Class|KismetSystemLibrary|UnPauseTimer (Variables|Interaction/Revive|GetPlayerYourReviving) "BleedOutTimer") ; Rsume Bleed Out
  (Utilities|Time|ClearTimerbyFunctionName 0 "RevivingPlayer")
  (Variables|Default|SetisBeingRevived? false)
  (if (Variables|Interaction/Revive|GetTouchingReviveTrigger?)
    _))

(event Custom|ServerTellPlayerToRevive
  (bind _playeryourreviving (Variables|Interaction/Revive|GetPlayerYourReviving))
  ;[0 1 0] Server Tells player your reviving to Revive.
  (Utilities|IsValid _playeryourreviving
    (:Is%20Valid
      (Utilities|Time|ClearTimerbyFunctionName 0 "RevivingPlayer")
      (CallFunction|ServerRevivePlayer _playeryourreviving)
      (Variables|Default|SetisBeingRevived? false))))

(event EventOnDeath
  (params (KillingDamage :type Float%20%28single-precision%29) (DamageEvent :type Damage%20Event%20Structure%20%28by%20ref%29) (InstigatingPawn :type Pawn%20Object%20Reference) (DamageCauser :type Actor%20Object%20Reference))
  (bind _playernamewidget (Variables|Default|GetPlayerNameWidget))
  ;[0 1 0] Player Health and Death
  (|CallParentFunction KillingDamage DamageEvent InstigatingPawn DamageCauser)
  (Utilities|IsValid _playernamewidget
    (:Is%20Valid
      (Components|DestroyComponent _playernamewidget)
      (Variables|PlayerVariables|SetIsDead? true)
      (bind _asbp_zmgame_mode (Utilities|Casting|CastToBP_ZMGameMode (Game|GetGameMode)))
      (Default|CheckforGameOver _asbp_zmgame_mode))))

(event EventBeginPlay
  ;[0.002197 0.907 1] Begin Play. Set character variables to the values entered into the character data table.
  (Variables|Interaction/Revive|SetBleedOutCounter (Variables|Interaction/Revive|GetBleedOutTime)))

(event EventPossessed
  (params (NewController :type Controller%20Object%20Reference))
  ;[0.002197 0.907 1] Begin Play. Set character variables to the values entered into the character data table.
  (|CallParentFunction NewController)
  (Utilities|FlowControl|Delay 0.2)
  (Class|DFBaseCharacter|GiveLoadout "/ZombieSurvival/Kits/Blue/HDKIT_Glock.HDKIT_Glock" true))

(event Game|Damage|EventAnyDamage
  (params (Damage :type Float%20%28single-precision%29) (DamageType :type Damage%20Type%20Object%20Reference) (InstigatedBy :type Controller%20Object%20Reference) (DamageCauser :type Actor%20Object%20Reference))
  ;[0 1 0] Player Health and Death
  (|CallParentFunction Damage DamageType InstigatedBy DamageCauser))

(event Input|KeyboardEvents|X
  (params (Key :type Key%20Structure))
  (:Pressed
    (CallFunction|EquipSelectedItemfromInventory true)))

(fn ConstructionScript)

(fn BleedOutTimer
  (bind _output_get (Variables|Interaction/Revive|SetBleedOutCounter (- (Variables|Interaction/Revive|GetBleedOutCounter) 1.0)))
  (if (<= _output_get 0.0) ; If True then you Bled Out.
    (CallFunction|PlayerHasDied)))

(fn OnRepBleedOutCounter
  (bind _aswbp_player_name_above_widget (Utilities|Casting|CastToWBP_PlayerNameAboveWidget (UserInterface|GetUserWidgetObject (Variables|Default|GetPlayerNameWidget))))
  (Rendering|Components|TextRender|SetText (Variables|/ZombieSurvival/Blueprints/Widgets/WBP_PlayerNameAboveWidget.WBP_PlayerNameAboveWidget_C|GetBleedOutTimer _aswbp_player_name_above_widget) (Utilities|Text|ToText(String) (Utilities|String|Append (Utilities|String|ToString(Integer) (Math|Float|Round (Variables|Interaction/Revive|GetBleedOutCounter))) "sec")))
  (Default|SetBleedOutColor _aswbp_player_name_above_widget (Variables|Interaction/Revive|GetBleedOutTime) (Variables|Interaction/Revive|GetBleedOutCounter)))

(fn RevivingPlayer
  (if (Variables|Interaction/Revive|GetIsDowned?)
    ;[1 1 1] If You Die While Reviving Someone, then cancle revive and hide revive widgets
    (CallFunction|ServerUnPauseBleedOutTimer) ; Server Resumes the Bleed Out Timer for the Downed Player
    (elif (Variables|Interaction/Revive|GetTouchingReviveTrigger?) ; If True Then Revive Player
      (CallFunction|ServerTellPlayertoRevive) ; Server Revives the Downed Player
      (CallFunction|ServerPauseBleedOutTime) ; Server Stops the Bleed Out Timer for the Downed Player
      (elif (Variables|Interaction/Revive|GetTouchingReviveTrigger?)
        (if (Variables|Interaction/Revive|GetUseButtonPressed?)
          (CallFunction|ServerPauseBleedOutTime) ; Server Stops the Bleed Out Timer for the Downed Player
          (else
            (CallFunction|ServerUnPauseBleedOutTimer :!label _label) ; Server Resumes the Bleed Out Timer for the Downed Player
          ))
        (else
          (goto _label))))))

(fn CalcInteractionTime
  (if (not (>= (Class|PlayerController|GetInputKeyTimeDown (Variables|PlayerVariables|GetMyPlayerController) (Variables|Interaction/Revive|GetInteractionKey)) (Variables|PickupVariables|GetPickupTime))) ; If True Then Interact with actor
    (if (not (Variables|Interaction/Revive|GetUseButtonPressed?))
      (Utilities|Time|ClearTimerbyFunctionName 0 "CalcInteractionTime"))))

(fn OnRepNameOfPlayer
  (if (not (Networking|IsDedicatedServer))
    (bind _returnvalue (UserInterface|CreateWidget "/ZombieSurvival/Blueprints/Widgets/WBP_PlayerNameAboveWidget.WBP_PlayerNameAboveWidget_C"))
    (UserInterface|SetWidget (Variables|Default|GetPlayerNameWidget) _returnvalue)
    (Default|SetName _returnvalue (Variables|PlayerVariables|GetNameOfPlayer))))

(fn OnRepIsBeingRevived?)