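; Player state for the ZM mode that keeps the scoreboard current and manages spectating after death.
; BeginPlay asks the game mode to update the scoreboard, and RepNotifies for points, kills, deaths and downs call for updates.
; Spectate events cycle the view through living player characters, updating the spectator HUD.
; A destroyed-actor binding advances to another player, falling back to a random GameOverCamera when no valid target remains.
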(event Custom|SpectateeDead
  (params (DestroyedActor :type Actor%20Object%20Reference))
  (bind _spectatorscontroller (Variables|Default|GetSpectatorsController))
  ;[1 1 1] When person you're spectating dies find another person to spectate
  (Utilities|IsValid _spectatorscontroller
    (:Is%20Valid
      (if (Variables|/ZombieSurvival/Core/BP_ZMPlayerController.BP_ZMPlayerController_C|GetIsSpectator? _spectatorscontroller)
        (Utilities|FlowControl|Delay 0.2)
        (Variables|Default|SetWhoYourSpectating 0)
        (CallFunction|SpectateNextPlayer _spectatorscontroller)))))

(event Custom|PushToUpdateScoreboard
  (bind _asbp_zmgame_mode (Utilities|Casting|CastToBP_ZMGameMode (Game|GetGameMode)))
  (Default|UpdateScoreboard _asbp_zmgame_mode))

(event Custom|SpectateNextPlayer
  (params (PlayerController :type Player%20Controller%20Object%20Reference))
  (bind _spectatorscontroller (Variables|Default|GetSpectatorsController))
  ;[1 1 1] Spectate Next Player
  (Utilities|IsValid PlayerController
    (:Is%20Valid
      (bind _asbp_zmplayer_controller (Utilities|Casting|CastToBP_ZMPlayerController PlayerController))
      (if (Variables|/ZombieSurvival/Core/BP_ZMPlayerController.BP_ZMPlayerController_C|GetIsSpectator? _asbp_zmplayer_controller)
        (bind _outactors (Actor|GetAllActorsOfClass "/ZombieSurvival/Core/BP_ZMPlayerCharacter.BP_ZMPlayerCharacter_C"))
        (bind _output_get (Variables|Default|SetArrayOfPlayersAlive _outactors))
        (Variables|Default|SetOldPersonYourSpectating (Utilities|Array|Get(acopy) _output_get (Variables|Default|GetCurrentIndexSpectator)))
        (if (>= (Variables|Default|GetCurrentIndexSpectator) (- (Utilities|Array|Length (Variables|Default|GetArrayOfPlayersAlive)) 1))
          (Variables|Default|SetCurrentIndexSpectator 0)
          (else
            (Variables|Default|SetCurrentIndexSpectator (+ (Variables|Default|GetCurrentIndexSpectator) 1))))
        (bind _output_get_2 (Variables|Default|SetWhoYourSpectating (Utilities|Array|Get(acopy) _output_get (Variables|Default|GetCurrentIndexSpectator))))
        (Game|Player|SetViewTargetwithBlend PlayerController _output_get_2 0.5 "VTBlend_Linear" 0.0 false)
        (Default|UpdateSpectatorHUD _asbp_zmplayer_controller (Variables|Default|GetWhoYourSpectating))
        (Utilities|IsValid (Variables|Default|GetWhoYourSpectating)
          (:Is%20Valid
            ;[1 1 1] When person you're spectating dies find another person to spectate
            (Game|BindEventtoOnDestroyed (Variables|Default|GetWhoYourSpectating) (delegate Custom|SpectateeDead))
            ;[1 1 1] Tell Spectators Controller to Locally Tell The SpectatorBP to bind an event to This player He's Spectating
            (bind _asbp_zmplayer_controller_2 (Utilities|Casting|CastToBP_ZMPlayerController (Components|GetOwner)))
            (Default|TellSpectatorWhoYourSpectating _asbp_zmplayer_controller_2 (Variables|Default|GetWhoYourSpectating) (Variables|Default|GetOldPersonYourSpectating)))
          (:Is%20Not%20Valid
            ;[1 1 1] If Everyone is dead then spectate a random Game Over Camera Actor (place these in the map wherever you like)
            (bind _outactors_2 (Actor|GetAllActorsOfClass "/ZombieSurvival/Blueprints/Blueprints/DownedBlueprints/GameOverCamera.GameOverCamera_C"))
            (Utilities|IsValid _spectatorscontroller
              (:Is%20Valid
                (Game|Player|SetViewTargetwithBlend _spectatorscontroller (Utilities|Array|Get(acopy) _outactors_2 (Math|Random|RandomInteger (Utilities|Array|Length _outactors_2))) 1.0 "VTBlend_Linear" 0.0 false)))))))))

(event Custom|SetWhoToSpectate
  (params (Controller :type Controller%20Object%20Reference))
  ;[1 1 1] Who To Spectate When You Die
  (Utilities|FlowControl|Delay 0.2)
  (bind _asbp_zmplayer_controller (Utilities|Casting|CastToBP_ZMPlayerController Controller))
  (if (Variables|/ZombieSurvival/Core/BP_ZMPlayerController.BP_ZMPlayerController_C|GetIsSpectator? _asbp_zmplayer_controller)
    (Variables|Default|SetSpectatorsController _asbp_zmplayer_controller)
    (bind _outactors (Actor|GetAllActorsOfClass "/ZombieSurvival/Core/BP_ZMPlayerCharacter.BP_ZMPlayerCharacter_C"))
    (bind _output_get (Variables|Default|SetArrayOfPlayersAlive _outactors))
    (Variables|Default|SetWhoYourSpectating (Utilities|Array|Get(acopy) _output_get (Variables|Default|GetCurrentIndexSpectator)))
    (Variables|Default|SetOldPersonYourSpectating 0)
    (Utilities|FlowControl|Delay 0.2)
    (Game|Player|SetViewTargetwithBlend (Variables|Default|GetSpectatorsController) (Variables|Default|GetWhoYourSpectating) 1.0 "VTBlend_Linear" 0.0 false)
    (Default|SetVisibilityPlayerHUDwhenSpectating (Variables|Default|GetSpectatorsController))
    (Default|UpdateSpectatorHUD (Variables|Default|GetSpectatorsController) (Variables|Default|GetWhoYourSpectating))
    (Utilities|IsValid (Variables|Default|GetWhoYourSpectating)
      (:Is%20Valid
        ;[1 1 1] When person you're spectating dies find another person to spectate
        (Game|BindEventtoOnDestroyed (Variables|Default|GetWhoYourSpectating) (delegate Custom|SpectateeDead))
        ;[1 1 1] Tell Spectators Controller to Locally Tell The SpectatorBP to bind an event to This player He's Spectating
        (bind _asbp_zmplayer_controller_2 (Utilities|Casting|CastToBP_ZMPlayerController (Components|GetOwner)))
        (Default|TellSpectatorWhoYourSpectating _asbp_zmplayer_controller_2 (Variables|Default|GetWhoYourSpectating) (Variables|Default|GetOldPersonYourSpectating)))
      (:Is%20Not%20Valid
        ;[1 1 1] If Everyone is dead then spectate a random Game Over Camera Actor (place these in the map wherever you like)
        (bind _outactors_2 (Actor|GetAllActorsOfClass "/ZombieSurvival/Blueprints/Blueprints/DownedBlueprints/GameOverCamera.GameOverCamera_C"))
        (Utilities|IsValid (Variables|Default|GetSpectatorsController)
          (:Is%20Valid
            (Game|Player|SetViewTargetwithBlend (Variables|Default|GetSpectatorsController) (Utilities|Array|Get(acopy) _outactors_2 (Math|Random|RandomInteger (Utilities|Array|Length _outactors_2))) 1.0 "VTBlend_Linear" 0.0 false)))))))

(event Custom|SpectatePreviousPlayer
  (params (PlayerController :type Player%20Controller%20Object%20Reference))
  (bind _spectatorscontroller (Variables|Default|GetSpectatorsController))
  ;[1 1 1] Spectate Previous Player
  (Utilities|IsValid PlayerController
    (:Is%20Valid
      (bind _asbp_zmplayer_controller (Utilities|Casting|CastToBP_ZMPlayerController PlayerController))
      (if (Variables|/ZombieSurvival/Core/BP_ZMPlayerController.BP_ZMPlayerController_C|GetIsSpectator? _asbp_zmplayer_controller)
        (bind _outactors (Actor|GetAllActorsOfClass "/ZombieSurvival/Core/BP_ZMPlayerCharacter.BP_ZMPlayerCharacter_C"))
        (bind _output_get (Variables|Default|SetArrayOfPlayersAlive _outactors))
        (Variables|Default|SetOldPersonYourSpectating (Utilities|Array|Get(acopy) _output_get (Variables|Default|GetCurrentIndexSpectator)))
        (if (== (Variables|Default|GetCurrentIndexSpectator) 0)
          (Variables|Default|SetCurrentIndexSpectator (- (Utilities|Array|Length (Variables|Default|GetArrayOfPlayersAlive)) 1))
          (else
            (Variables|Default|SetCurrentIndexSpectator (- (Variables|Default|GetCurrentIndexSpectator) 1))))
        (bind _output_get_2 (Variables|Default|SetWhoYourSpectating (Utilities|Array|Get(acopy) _output_get (Variables|Default|GetCurrentIndexSpectator))))
        (Game|Player|SetViewTargetwithBlend PlayerController _output_get_2 0.5 "VTBlend_Linear" 0.0 false)
        (Default|UpdateSpectatorHUD _asbp_zmplayer_controller (Variables|Default|GetWhoYourSpectating))
        (Utilities|IsValid (Variables|Default|GetWhoYourSpectating)
          (:Is%20Valid
            ;[1 1 1] When person you're spectating dies find another person to spectate
            (Game|BindEventtoOnDestroyed (Variables|Default|GetWhoYourSpectating) (delegate Custom|SpectateeDead))
            ;[1 1 1] Tell Spectators Controller to Locally Tell The SpectatorBP to bind an event to This player He's Spectating
            (bind _asbp_zmplayer_controller_2 (Utilities|Casting|CastToBP_ZMPlayerController (Components|GetOwner)))
            (Default|TellSpectatorWhoYourSpectating _asbp_zmplayer_controller_2 (Variables|Default|GetWhoYourSpectating) (Variables|Default|GetOldPersonYourSpectating)))
          (:Is%20Not%20Valid
            ;[1 1 1] If Everyone is dead then spectate a random Game Over Camera Actor (place these in the map wherever you like)
            (bind _outactors_2 (Actor|GetAllActorsOfClass "/ZombieSurvival/Blueprints/Blueprints/DownedBlueprints/GameOverCamera.GameOverCamera_C"))
            (Utilities|IsValid _spectatorscontroller
              (:Is%20Valid
                (Game|Player|SetViewTargetwithBlend _spectatorscontroller (Utilities|Array|Get(acopy) _outactors_2 (Math|Random|RandomInteger (Utilities|Array|Length _outactors_2))) 1.0 "VTBlend_Linear" 0.0 false)))))))))

(event EventBeginPlay
  (CallFunction|PushtoUpdateScoreboard))

(fn ConstructionScript)

(fn OnRepPlayerPoints
  (Default|CallUpdateScoreboard))

(fn OnRepPlayerDeaths
  (Default|CallUpdateScoreboard))

(fn OnRepPlayerKills
  (Default|CallUpdateScoreboard))

(fn OnRepPlayerDowns
  (Default|CallUpdateScoreboard))