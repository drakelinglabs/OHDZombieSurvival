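; Game state for the zombie mode that relays wave status, powerup effects and game-over display to player controllers.
; A looping timer copies zombie, wave and player counters from BP_ZMGameMode, mainly to debug the zombie counter.
; Events push notification text to a player's HUD and set or reset the Quad Points multiplier and timer widget for all players.
; Game over creates each controller's scoreboard widget and has the game mode update it.
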(event Custom|NotificationText
  (params (NotificationText :type Text) (PlayerController :type Player%20Controller%20Object%20Reference) (Lifetime :type Float%20%28single-precision%29))
  ;[1 1 1] Notification Text such as Max ammo, double points, etc
  (bind _asbp_zmplayer_controller (Utilities|Casting|CastToBP_ZMPlayerController PlayerController))
  (Utilities|IsValid (Variables|/ZombieSurvival/Core/BP_ZMPlayerController.BP_ZMPlayerController_C|GetHUDWidgetReference _asbp_zmplayer_controller)
    (:Is%20Valid
      (Default|SetNotificationText (Variables|/ZombieSurvival/Core/BP_ZMPlayerController.BP_ZMPlayerController_C|GetHUDWidgetReference _asbp_zmplayer_controller) NotificationText Lifetime))))

(event Custom|CreateGameOverWidget
  (params (AllPlayerControllers :type Array%20of%20Player%20Controller%20Object%20References))
  ;[1 1 1] Create Game Over Widget for all player controllers as well as show the scoreboard
  (for _array_element AllPlayerControllers
    (bind _asbp_zmplayer_controller (Utilities|Casting|CastToBP_ZMPlayerController _array_element))
    (Default|CreateScoreboardWidget _asbp_zmplayer_controller)
    (bind _asbp_zmgame_mode (Utilities|Casting|CastToBP_ZMGameMode (Game|GetGameMode)))
    (Default|UpdateScoreboard _asbp_zmgame_mode)))

(event Custom|UpdateZombieCounter
  ;[1 1 1] Used for Zombie Counter Debuging. Can Remove if you don't want zombie counter
  (bind _asbp_zmgame_mode (Utilities|Casting|CastToBP_ZMGameMode (Game|GetGameMode)))
  (Variables|DebugVariables|SetNumZombsLeft (Variables|/ZombieSurvival/Core/BP_ZMGameMode.BP_ZMGameMode_C|GetZombsLeftCounter _asbp_zmgame_mode))
  (Variables|DebugVariables|SetNumZombsAlive (Variables|/ZombieSurvival/Core/BP_ZMGameMode.BP_ZMGameMode_C|GetZombsAliveCounter _asbp_zmgame_mode))
  (Variables|DebugVariables|SetNumZombsPerWave (Variables|/ZombieSurvival/Core/BP_ZMGameMode.BP_ZMGameMode_C|GetNumZombiesPerWave _asbp_zmgame_mode))
  (Variables|DebugVariables|SetZombSpawnCounter (Variables|/ZombieSurvival/Core/BP_ZMGameMode.BP_ZMGameMode_C|GetZombsSpawnCounter _asbp_zmgame_mode))
  (Variables|DebugVariables|SetNumberOfPlayers (Variables|/ZombieSurvival/Core/BP_ZMGameMode.BP_ZMGameMode_C|GetNumberOfPlayers _asbp_zmgame_mode)))

(event Custom|SetupQuadPoints
  (params (AllPlayerControllers :type Array%20of%20Player%20Controller%20Object%20References) (TimePowerupLasts :type Integer) (PointsMultiplier :type Integer))
  ;[1 1 1] Quad Points Powerup
  (Variables|Default|SetTimePowerupLasts TimePowerupLasts)
  (for _array_element AllPlayerControllers
    (bind _asbp_zmplayer_controller (Utilities|Casting|CastToBP_ZMPlayerController _array_element))
    (Variables|/ZombieSurvival/Core/BP_ZMPlayerController.BP_ZMPlayerController_C|SetPointMultiplier _asbp_zmplayer_controller PointsMultiplier)
    (Utilities|IsValid (Variables|/ZombieSurvival/Core/BP_ZMPlayerController.BP_ZMPlayerController_C|GetHUDWidgetReference _asbp_zmplayer_controller)
      (:Is%20Valid
        (Widget|SetVisibility (Variables|/ZombieSurvival/Blueprints/Widgets/HUD/PlayerHUDWidget.PlayerHUDWidget_C|GetPowerUpTimer (Variables|/ZombieSurvival/Core/BP_ZMPlayerController.BP_ZMPlayerController_C|GetHUDWidgetReference _asbp_zmplayer_controller)) "Visible")))))

(event Custom|EndQuadPoints
  (params (AllPlayerControllers :type Array%20of%20Player%20Controller%20Object%20References))
  ;[1 1 1] Quad Points Powerup
  (for _array_element AllPlayerControllers
    (bind _asbp_zmplayer_controller (Utilities|Casting|CastToBP_ZMPlayerController _array_element))
    (Utilities|IsValid (Variables|/ZombieSurvival/Core/BP_ZMPlayerController.BP_ZMPlayerController_C|GetHUDWidgetReference _asbp_zmplayer_controller)
      (:Is%20Valid
        (Widget|SetVisibility (Variables|/ZombieSurvival/Blueprints/Widgets/HUD/PlayerHUDWidget.PlayerHUDWidget_C|GetPowerUpTimer (Variables|/ZombieSurvival/Core/BP_ZMPlayerController.BP_ZMPlayerController_C|GetHUDWidgetReference _asbp_zmplayer_controller)) "Collapsed"))
      (:Is%20Not%20Valid
        _))
    (Variables|/ZombieSurvival/Core/BP_ZMPlayerController.BP_ZMPlayerController_C|SetPointMultiplier _asbp_zmplayer_controller 1)))

(event EventBeginPlay
  (|CallParentFunction)
  (Utilities|Time|SetTimerbyEvent (delegate Custom|UpdateZombieCounter) 0.1 true))

(fn ConstructionScript)