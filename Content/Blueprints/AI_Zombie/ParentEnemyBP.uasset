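; Base enemy Blueprint for zombies that keeps the game mode's wave zombie count accurate.
; On BeginPlay, enemies that count toward the wave total bind to their own OnDestroyed event.
; If destroyed without dying normally, such as by a kill zone, the enemy tells BP_ZMGameMode to decrement its zombie counter, guarded by IsDead as a fallback to normal death logic.
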(event Custom|SubtractFromZombsRemaining
  (params (DestroyedActor :type Actor%20Object%20Reference))
  ;[1 1 1] Decrement Number of Zombies left when destroyed if for some reason he didn't when he died. (This is a double check)
  (CallFunction|ServerDecrementNumZombsRemaining))

(event Custom|ServerDecrementNumZombsRemaining
  ;[1 1 1] Decrements the Zombie Counter in Game Mode if a zombie Dies "unaturally" meaning he was destroyed instead of executing his death logic. Used as a check just incase. For example if a zombie fell out of the map and got destroyed by the kill zone his normal death logic wouldn't execute so the zombie counter wouldn't decrease in gamemode. But his will prevent that by simply doing it here.
  (if (not (Variables|Default|GetIsDead?))
    (bind _asbp_zmgame_mode (Utilities|Casting|CastToBP_ZMGameMode (Game|GetGameMode)))
    (Default|DecrementZombieCounter _asbp_zmgame_mode self)))

(event EventBeginPlay
  ;[1 1 1] Begin Play
  (if (Variables|Default|GetCountTowardsWaveTotal?) ; Does enemy count towards the wave total zombies? (ex: boss might not want to)
    ;[1 1 1] Decrement Number of Zombies left when destroyed if for some reason he didn't when he died. (This is a double check)
    (EventDispatchers|BindEventtoOnDestroyed (delegate Custom|SubtractFromZombsRemaining))))

(fn ConstructionScript)