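; Master gib chunk actor for zombie gibbing: a short-lived piece of flung body part with a blood effect.
; On BeginPlay it randomizes the arm mesh's scale per axis and applies a random upward and sideways world-space impulse at the actor's location.
; After a short delay it deactivates the blood FX and sets a random lifespan so the chunk cleans itself up.
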(event EventBeginPlay
  (bind _returnvalue (Math|Random|RandomFloatinRange 0.9 1.1))
  (Transformation|SetWorldScale3D (Variables|Default|GetSK_ZombieBB_ArmL_V1) (Math|Vector|MakeVector _returnvalue _returnvalue _returnvalue))
  (Physics|AddImpulseatLocation (Variables|Default|GetSK_ZombieBB_ArmL_V1) (* (Math|Vector|MakeVector 0.0 (Math|Random|RandomFloatinRange -1e+02 1e+02) (Math|Random|RandomFloatinRange 5e+01 1e+02)) 5.0) (Transformation|GetActorLocation) "None")
  (Utilities|FlowControl|Delay 2.0)
  (Components|Activation|Deactivate (Variables|Default|GetBloodFX))
  (Actor|SetLifeSpan (Math|Random|RandomFloatinRange 3.0 6.0)))

(fn ConstructionScript)