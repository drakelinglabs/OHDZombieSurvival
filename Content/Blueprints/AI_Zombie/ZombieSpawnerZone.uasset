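; ZombieSpawnerZone is a box volume that spawns random zombie types for the wave-based zombie game mode.
; SpawnZombie lazily caches BP_ZMGameMode, then checks that the zone is activatable, the wave is running and the alive cap is not reached.
; It passes a random enemy type and point inside the box to the game mode's SpawnZombie.
; Once the wave's spawn quota is met, it clears its own SpawnZombie timer.
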(fn ConstructionScript)

(fn SpawnZombie
  (bind _spawnerzone (Variables|Default|GetSpawnerZone))
  (Utilities|IsValid (Variables|Default|GetGamemodeREF)
    (:Is%20Valid
      _)
    (:Is%20Not%20Valid
      (bind _asbp_zmgame_mode (Utilities|Casting|CastToBP_ZMGameMode (Game|GetGameMode)))
      (Variables|Default|SetGamemodeREF _asbp_zmgame_mode)))
  (Variables|Default|SetEnemyToSpawn (Utilities|Array|Get(acopy) (Variables|Default|GetTypeOfEnemyToSpawn) (Math|Random|RandomIntegerinRange 0 (- (Utilities|Array|Length (Variables|Default|GetTypeOfEnemyToSpawn)) 1))))
  (if (and (Variables|Default|GetCanBeActivatedYet?) (not (Variables|/ZombieSurvival/Core/BP_ZMGameMode.BP_ZMGameMode_C|GetWaveOver? (Variables|Default|GetGamemodeREF))))
    (if (< (Variables|/ZombieSurvival/Core/BP_ZMGameMode.BP_ZMGameMode_C|GetZombsAliveCounter (Variables|Default|GetGamemodeREF)) (Variables|/ZombieSurvival/Core/BP_ZMGameMode.BP_ZMGameMode_C|GetMaxNumZombsAtOnce (Variables|Default|GetGamemodeREF)))
      (if (< (Variables|/ZombieSurvival/Core/BP_ZMGameMode.BP_ZMGameMode_C|GetZombsSpawnCounter (Variables|Default|GetGamemodeREF)) (Variables|/ZombieSurvival/Core/BP_ZMGameMode.BP_ZMGameMode_C|GetNumZombiesPerWave (Variables|Default|GetGamemodeREF)))
        (Default|SpawnZombie (Variables|Default|GetGamemodeREF) (Variables|Default|GetEnemyToSpawn) (Math|Random|RandomPointinBoundingBox (Transformation|GetWorldLocation _spawnerzone) (Components|Box|GetScaledBoxExtent _spawnerzone)))
        (else
          (Utilities|Time|ClearTimerbyFunctionName self "SpawnZombie"))))))