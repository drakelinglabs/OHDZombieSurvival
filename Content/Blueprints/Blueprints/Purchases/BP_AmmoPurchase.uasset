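; Ammo purchase that refills the buyer's weapons when bought, running the parent ServerPurchase and then ReplenishAmmo.
; ReplenishAmmo scans inventory weapons other than itself that have no replenishment delay, then stores enough of each one's first supported clip type to cover its shortfall from starting clips.
; CheckForAmmo applies the same eligibility test, but its only call sits in unconnected event logic and its visible return is always false.
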(event EventServerPurchase
  (params (PersonBuyingAmmo :type BP%20ZM%20Player%20Character%20Object%20Reference))
  (|CallParentFunction PersonBuyingAmmo)
  (CallFunction|ReplenishAmmo PersonBuyingAmmo))

(fn ConstructionScript
  (|CallParentFunction))

(fn ReplenishAmmo
  (params (Pawn :type BP%20ZM%20Player%20Character%20Object%20Reference))
  (bind _inventory (Variables|/Script/DonkehFramework.DFBaseCharacter|GetInventory Pawn))
  (Utilities|IsValid Pawn
    (:Is%20Valid
      (for _array_element (Variables|/Script/DonkehFramework.DFInventoryComponent|GetItems _inventory)
        (Utilities|IsValid _array_element
          (:Is%20Valid
            (bind _ashdbase_weapon (Utilities|Casting|CastToHDBaseWeapon _array_element))
            (if (Math|Boolean|ANDBoolean (!= _ashdbase_weapon self) (<= (Variables|/Script/HDMain.HDBaseWeapon|GetAmmoReplenishmentDelay _ashdbase_weapon) 0.0) (> (- (Variables|/Script/DonkehFramework.DFBaseGun|GetStartingAmmoClips _ashdbase_weapon) (Class|DFBaseGun|GetNumFreeAmmoClips _ashdbase_weapon false true)) 0) (> (Utilities|Set|Length (Variables|/Script/DonkehFramework.DFBaseGun|GetSupportedAmmoClips _ashdbase_weapon)) 0)) ; Check if the pawn should receive\nmore ammo for this weapon
              (bind _result (Utilities|Set|ToArray (Variables|/Script/DonkehFramework.DFBaseGun|GetSupportedAmmoClips _ashdbase_weapon)))
              (Class|DFBaseAmmoClip|StoreAmmoinInventory _inventory (* (Utilities|GetClassDefaults (Utilities|Array|Get(acopy) _result)) (- (Variables|/Script/DonkehFramework.DFBaseGun|GetStartingAmmoClips _ashdbase_weapon) (Class|DFBaseGun|GetNumFreeAmmoClips _ashdbase_weapon false true))) (Utilities|Array|Get(acopy) _result))
              (Math|Integer|IncrementInt (LocalVariables|GetNumberOfClipsRestored))))))
      (return (LocalVariables|GetNumberOfClipsRestored)))))

(fn CheckforAmmo
  (params (Pawn :type BP%20ZM%20Player%20Character%20Object%20Reference))
  (Utilities|IsValid Pawn
    (:Is%20Valid
      (Utilities|Array|Clear (LocalVariables|GetAddAmmo?))
      (for _array_element (Variables|/Script/DonkehFramework.DFInventoryComponent|GetItems (Variables|/Script/DonkehFramework.DFBaseCharacter|GetInventory Pawn))
        (Utilities|IsValid _array_element
          (:Is%20Valid
            (bind _ashdbase_weapon (Utilities|Casting|CastToHDBaseWeapon _array_element))
            (Utilities|Array|AddUnique (LocalVariables|GetAddAmmo?) (Math|Boolean|ANDBoolean (!= _ashdbase_weapon self) (<= (Variables|/Script/HDMain.HDBaseWeapon|GetAmmoReplenishmentDelay _ashdbase_weapon) 0.0) (> (- (Variables|/Script/DonkehFramework.DFBaseGun|GetStartingAmmoClips _ashdbase_weapon) (Class|DFBaseGun|GetNumFreeAmmoClips _ashdbase_weapon false true)) 0) (> (Utilities|Set|Length (Variables|/Script/DonkehFramework.DFBaseGun|GetSupportedAmmoClips _ashdbase_weapon)) 0))))))
      (bind _array_element_2 (Utilities|Array|ForEachLoopwithBreak (LocalVariables|GetAddAmmo?) :!label _label)
        (:LoopBody
          (if (not _array_element_2)
            (goto _label Break)))
        (:Completed
          (return false))))))