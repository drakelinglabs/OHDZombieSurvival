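; Master purchase station Blueprint for the zombie mode, handling the point cost of a buyable.
; Entering its box trigger shows a HUD hint with the cost and resets a DoOnce gate; leaving clears the hint.
; Used passes through that gate to ServerPurchase, allowing one attempt per trigger entry.
; ServerPurchase checks the player's points, deducts the cost and plays the purchase sound, but grants no item itself.
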(event OnComponentBeginOverlap(BoxTrigger)
  (params (OverlappedComponent :type Primitive%20Component%20Object%20Reference) (OtherActor :type Actor%20Object%20Reference) (OtherComp :type Primitive%20Component%20Object%20Reference) (OtherBodyIndex :type Integer) (bFromSweep :type Boolean) (SweepResult :type Hit%20Result%20Structure%20%28by%20ref%29))
  (bind _asbp_zmplayer_character (Utilities|Casting|CastToBP_ZMPlayerCharacter OtherActor))
  (CallFunction|ResetInteraction)
  (Variables|/ZombieSurvival/Core/BP_ZMPlayerCharacter.BP_ZMPlayerCharacter_C|SetShowHintstrings? _asbp_zmplayer_character true)
  (bind _asbp_zmplayer_controller (Utilities|Casting|CastToBP_ZMPlayerController (Pawn|GetController _asbp_zmplayer_character)))
  (Utilities|IsValid (Variables|/ZombieSurvival/Core/BP_ZMPlayerController.BP_ZMPlayerController_C|GetHUDWidgetReference _asbp_zmplayer_controller)
    (:Is%20Valid
      (Default|SetHintstring (Variables|/ZombieSurvival/Core/BP_ZMPlayerController.BP_ZMPlayerController_C|GetHUDWidgetReference _asbp_zmplayer_controller) (Utilities|Text|ToText(String) (Utilities|String|Append (Utilities|String|ToString(Text) (Variables|Default|GetHintstring)) " " (Utilities|String|ToString(Integer) (Variables|Default|GetCost)) " Points"))))))

(event OnComponentEndOverlap(BoxTrigger)
  (params (OverlappedComponent :type Primitive%20Component%20Object%20Reference) (OtherActor :type Actor%20Object%20Reference) (OtherComp :type Primitive%20Component%20Object%20Reference) (OtherBodyIndex :type Integer))
  (bind _asbp_zmplayer_character (Utilities|Casting|CastToBP_ZMPlayerCharacter OtherActor))
  (Variables|/ZombieSurvival/Core/BP_ZMPlayerCharacter.BP_ZMPlayerCharacter_C|SetShowHintstrings? _asbp_zmplayer_character false)
  (bind _asbp_zmplayer_controller (Utilities|Casting|CastToBP_ZMPlayerController (Pawn|GetController _asbp_zmplayer_character)))
  (Utilities|IsValid (Variables|/ZombieSurvival/Core/BP_ZMPlayerController.BP_ZMPlayerController_C|GetHUDWidgetReference _asbp_zmplayer_controller)
    (:Is%20Valid
      (Default|SetHintstring (Variables|/ZombieSurvival/Core/BP_ZMPlayerController.BP_ZMPlayerController_C|GetHUDWidgetReference _asbp_zmplayer_controller)))))

(event Custom|ResetInteraction
  (Utilities|FlowControl|DoOnce false) ; enters at Reset
)

(event Custom|ServerPurchase
  (params (PersonBuyingAmmo :type BP%20ZM%20Player%20Character%20Object%20Reference))
  (bind _asbp_zmplayer_controller (Utilities|Casting|CastToBP_ZMPlayerController (Pawn|GetController PersonBuyingAmmo)))
  (if (>= (Variables|/ZombieSurvival/Core/BP_ZMPlayerController.BP_ZMPlayerController_C|GetPoints _asbp_zmplayer_controller) (Variables|Default|GetCost)) ; Do You Have Enough Points?
    (Default|RemovePoints _asbp_zmplayer_controller (Variables|Default|GetCost))
    (Default|PlaySoundonPlayer PersonBuyingAmmo (Variables|Default|GetPurchaseSound))))

(event EventUsed
  (params (Invoker :type Actor%20Object%20Reference))
  (bind _asbp_zmplayer_character (Utilities|Casting|CastToBP_ZMPlayerCharacter Invoker))
  (Utilities|FlowControl|DoOnce false
    (:Completed
      (CallFunction|ServerPurchase _asbp_zmplayer_character))))

(fn ConstructionScript)