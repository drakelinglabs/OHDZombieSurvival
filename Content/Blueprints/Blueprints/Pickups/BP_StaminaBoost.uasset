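; BP_StaminaBoost is a pickup that changes the player character's maximum sprint and jump stamina.
; It extends the parent pickup logic, then resolves the player controller and character through the owning actor's instigator.
; It overwrites both max stamina values on the DFCharacterMovement component with the pickup's reward variables, rather than adding to them.
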(event EventPickupFunctionality
  (params (OwningActor :type BP%20ZM%20Player%20Character%20Object%20Reference))
  (|CallParentFunction OwningActor)
  (bind _asbp_zmplayer_controller (Utilities|Casting|CastToBP_ZMPlayerController (Pawn|GetController (Variables|/Script/Engine.Actor|GetInstigator OwningActor))))
  (bind _asbp_zmplayer_character (Utilities|Casting|CastToBP_ZMPlayerCharacter (Pawn|GetControlledPawn _asbp_zmplayer_controller)))
  (Variables|/Script/DonkehFramework.DFCharacterMovementComponent|SetSprintMaxStamina (Variables|/Script/DonkehFramework.DFBaseCharacter|GetDFCharacterMovement _asbp_zmplayer_character) (Variables|Default|GetSprintStaminaRewarded))
  (Variables|/Script/DonkehFramework.DFCharacterMovementComponent|SetJumpMaxStamina (Variables|/Script/DonkehFramework.DFBaseCharacter|GetDFCharacterMovement _asbp_zmplayer_character) (Variables|Default|GetJumpStaminaRewarded)))

(fn ConstructionScript
  (|CallParentFunction))