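; BP_DoublePointsPickup is a zombie-mode powerup pickup that temporarily multiplies points earned.
; It overrides the parent PickupFunctionality event, calls the parent logic, then casts the game mode to BP_ZMGameMode.
; It passes its notification text, notification lifetime, powerup duration and multiplier to the game mode's PointsMultiplierPowerup, which owns the effect.
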(event EventBeginPlay
  (|CallParentFunction) ; This node is disabled and will not be called.\nDrag off pins to build functionality.
)

(event EventPickupFunctionality
  (params (OwningActor :type BP%20ZM%20Player%20Character%20Object%20Reference))
  (|CallParentFunction OwningActor)
  (bind _asbp_zmgame_mode (Utilities|Casting|CastToBP_ZMGameMode (Game|GetGameMode)))
  (Default|PointsMultiplierPowerup _asbp_zmgame_mode (Variables|Default|GetNotificationText) (Variables|Default|GetLifeOfNotification) (Variables|Default|GetTimePowerupLasts) (Variables|Default|GetPointsMultiplier)))

(fn ConstructionScript
  (|CallParentFunction))