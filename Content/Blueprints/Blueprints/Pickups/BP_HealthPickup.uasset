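; Health pickup Blueprint that restores health to the actor it is given.
; It extends the parent's PickupFunctionality event, then checks that the owning actor is valid and alive.
; It adds HealthRewarded to that actor's Health, clamped between zero and MaxHealth.
; It then calls EventResetHealthEffect on the actor, a step marked as a hack.
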(event EventBeginPlay
  (|CallParentFunction) ; This node is disabled and will not be called.\nDrag off pins to build functionality.
)

(event EventPickupFunctionality
  (params (OwningActor :type BP%20ZM%20Player%20Character%20Object%20Reference))
  (|CallParentFunction OwningActor)
  (Utilities|IsValid OwningActor
    (:Is%20Valid
      (if (Class|DFBaseCharacter|IsAlive OwningActor)
        (Variables|/Script/DonkehFramework.DFBaseCharacter|SetHealth OwningActor (Math|Float|Clamp(Float) (+ (Variables|Default|GetHealthRewarded) (Variables|/Script/DonkehFramework.DFBaseCharacter|GetHealth OwningActor)) 0.0 (Variables|/Script/DonkehFramework.DFBaseCharacter|GetMaxHealth OwningActor)))
        ;[1 0.903 0] @HACK
        (Default|EventResetHealthEffect OwningActor)))))

(fn ConstructionScript
  (|CallParentFunction))