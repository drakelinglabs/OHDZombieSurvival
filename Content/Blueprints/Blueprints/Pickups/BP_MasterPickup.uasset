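; BP_MasterPickup is a base pickup that a player character collects by overlapping its trigger sphere, with an optional lifespan for zombie drops.
; The first player overlap wakes net dormancy and calls PickupFunctionality, which here sends a notification through the ZM game mode.
; It then multicasts, via a server event when lacking authority, the particle effect, sound and actor destruction.
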(event OnComponentBeginOverlap(SphereTrigger)
  (params (OverlappedComponent :type Primitive%20Component%20Object%20Reference) (OtherActor :type Actor%20Object%20Reference) (OtherComp :type Primitive%20Component%20Object%20Reference) (OtherBodyIndex :type Integer) (bFromSweep :type Boolean) (SweepResult :type Hit%20Result%20Structure%20%28by%20ref%29))
  ;[1 1 1] Overal Event
  (bind _asbp_zmplayer_character (Utilities|Casting|CastToBP_ZMPlayerCharacter OtherActor))
  (Networking|SetNetDormancy "DORM_Awake")
  (Utilities|FlowControl|DoOnce false
    (:Completed
      (CallFunction|PickupFunctionality _asbp_zmplayer_character)
      (Networking|SwitchHasAuthority
        (:Authority
          (CallFunction|MulticastPickupPowerup))
        (:Remote
          (CallFunction|ServerPickupPowerup))))))

(event Custom|ServerPickupPowerup
  ;[1 1 1] Pickup Visual Effects
  (CallFunction|MulticastPickupPowerup))

(event Custom|MulticastPickupPowerup
  (bind _returnvalue (Transformation|GetActorLocation))
  ;[1 1 1] Pickup Visual Effects
  (Effects|SpawnEmitteratLocation (Variables|Effects|GetPickupParticleEffect) _returnvalue)
  (Audio|PlaySoundatLocation (Variables|Effects|GetPickupSound) _returnvalue "0, 0, 0" 1.0 1.0 0.0 0 0 0)
  (Actor|DestroyActor))

(event Custom|PickupFunctionality
  (params (OwningActor :type BP%20ZM%20Player%20Character%20Object%20Reference))
  ;[1 1 1] Functionlity
  (bind _asbp_zmgame_mode (Utilities|Casting|CastToBP_ZMGameMode (Game|GetGameMode)))
  (Default|SendNotificationText _asbp_zmgame_mode (Variables|Notification|GetNotificationText) (Variables|Notification|GetLifeOfNotification)))

(event EventBeginPlay
  ;[1 1 1] Life span
  (if (Variables|Default|GetZombieDrop)
    (Actor|SetLifeSpan (Variables|Default|GetPickupLifeSpan))))

(fn ConstructionScript)